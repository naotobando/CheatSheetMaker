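; BP_CheatSheet shows an on-screen cheat sheet of commands with their descriptions.
; On BeginPlay it creates a WB_CS_ListView widget, adds it to the viewport hidden, and registers its own toggle shortcut as an entry.
; The AddCommand event forwards each entry to the widget's list.
; Shift+SpaceBar drives a FlipFlop that alternately shows and hides the widget.
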(event Custom|AddCommand
  (params (Command :type String) (Description :type String) (DisplayName :type String))
  (Default|AddList (Variables|Default|GetWB_CS_ListView) Command Description DisplayName))

(event EventBeginPlay
  (Utilities|FlowControl|Sequence
    (:then_0
      (bind _returnvalue (UserInterface|CreateWidget "/CheatSheetMaker/WB_CS_ListView.WB_CS_ListView_C" (Game|GetPlayerController 0)))
      (bind _output_get (Variables|Default|SetWB_CS_ListView _returnvalue))
      (UserInterface|Viewport|AddtoViewport _output_get 0))
    (:then_1
      (Widget|SetVisibility (Variables|Default|GetWB_CS_ListView) "Hidden"))
    (:then_2
      (Utilities|AddCommand "Shift + SpaceBar" "Switch Visibility of CheatSheet" self))))

(event Input|KeyboardEvents|ShiftSpaceBar
  (params (Key :type Key%20Structure :default "None"))
  (bind _wb_cs_listview (Variables|Default|GetWB_CS_ListView))
  (:Pressed
    (Utilities|FlowControl|FlipFlop
      (:A
        (Widget|SetVisibility _wb_cs_listview "Visible"))
      (:B
        (Widget|SetVisibility _wb_cs_listview "Hidden")))))

(fn ConstructionScript)